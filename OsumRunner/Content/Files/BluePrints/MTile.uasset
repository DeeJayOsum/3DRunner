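; MTile is a track tile for a three-lane runner that spawns its own lane contents and keeps the track going.
; On BeginPlay, a random roll may place a Pipe, Box or CoinPickup in one lane, or leave the tile empty.
; When the player character overlaps its Box trigger, it asks the GameMode for another tile, adds multiplied points, raises walk speed within a clamp and destroys itself after a short delay.
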(event OnComponentBeginOverlap(Box)
  (params (OverlappedComponent :type Primitive%20Component%20Object%20Reference) (OtherActor :type Actor%20Object%20Reference) (OtherComp :type Primitive%20Component%20Object%20Reference) (OtherBodyIndex :type Integer) (bFromSweep :type Boolean) (SweepResult :type Hit%20Result%20Structure%20%28by%20ref%29))
  (Utilities|Casting|CastToThirdPersonCharacter OtherActor)
  (bind _asthird_person_game_mode (Utilities|Casting|CastToThirdPersonGameMode (Game|GetGameMode)))
  (Default|SpawnTile _asthird_person_game_mode)
  (bind _asthird_person_game_mode_2 (Utilities|Casting|CastToThirdPersonGameMode (Game|GetGameMode)))
  (Variables|/Game/ThirdPersonBP/Blueprints/ThirdPersonGameMode.ThirdPersonGameMode_C|SetCurrentPoints _asthird_person_game_mode_2 (+ (* 1 (Variables|/Game/ThirdPersonBP/Blueprints/ThirdPersonGameMode.ThirdPersonGameMode_C|GetPointMultiplier _asthird_person_game_mode_2)) (Variables|/Game/ThirdPersonBP/Blueprints/ThirdPersonGameMode.ThirdPersonGameMode_C|GetCurrentPoints _asthird_person_game_mode_2)))
  (bind _asthird_person_character (Utilities|Casting|CastToThirdPersonCharacter (Game|GetPlayerCharacter 0)))
  (Variables|/Script/Engine.CharacterMovementComponent|SetMaxWalkSpeed (Variables|/Script/Engine.Character|GetCharacterMovement _asthird_person_character) (Math|Float|Clamp(Float) (* (Variables|/Script/Engine.CharacterMovementComponent|GetMaxWalkSpeed (Variables|/Script/Engine.Character|GetCharacterMovement _asthird_person_character)) 1.1) 6e+02 3e+03))
  (Utilities|FlowControl|Delay 0.5)
  (Actor|DestroyActor))

(event EventBeginPlay
  (CallFunction|SpawnPipe))

(event Collision|EventActorBeginOverlap
  (params (OtherActor :type Actor%20Object%20Reference)))

(event EventTick
  (params (DeltaSeconds :type Float%20%28single-precision%29)))

(fn ConstructionScript)

(fn SpawnPipe
  (bind _lane0 (Variables|Default|GetLane0))
  (bind _lane1 (Variables|Default|GetLane1))
  (bind _lane2 (Variables|Default|GetLane2))
  (bind _returnvalue (Transformation|GetWorldTransform _lane2))
  (bind _returnvalue_2 (Transformation|GetWorldTransform _lane0))
  (bind _returnvalue_3 (Transformation|GetWorldTransform _lane1))
  (switch int (Math|Random|RandomIntegerinRange 0 20)
    (:0
      (Game|SpawnActorfromClass "/Game/Files/BluePrints/Pipe.Pipe_C" _returnvalue_2 "Undefined" 0 0))
    (:1
      (Game|SpawnActorfromClass "/Game/Files/BluePrints/Pipe.Pipe_C" _returnvalue_3 "Undefined" 0 0))
    (:2
      (Game|SpawnActorfromClass "/Game/Files/BluePrints/Pipe.Pipe_C" _returnvalue "Undefined" 0 0))
    (:15
      (Game|SpawnActorfromClass "/Game/Files/BluePrints/Box.Box_C" _returnvalue_2 "Undefined" 0 0))
    (:16
      (Game|SpawnActorfromClass "/Game/Files/BluePrints/Box.Box_C" _returnvalue "Undefined" 0 0))
    (:17
      (Game|SpawnActorfromClass "/Game/Files/BluePrints/Box.Box_C" _returnvalue_3 "Undefined" 0 0))
    (:18
      (Game|SpawnActorfromClass "/Game/Files/BluePrints/CoinPickup.CoinPickup_C" _returnvalue_2 "Undefined" 0 0))
    (:19
      (Game|SpawnActorfromClass "/Game/Files/BluePrints/CoinPickup.CoinPickup_C" _returnvalue "Undefined" 0 0))
    (:20
      (Game|SpawnActorfromClass "/Game/Files/BluePrints/CoinPickup.CoinPickup_C" _returnvalue_3 "Undefined" 0 0))))